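; TimeControl_BP is a component intended to let an object rewind through its past transforms.
; On BeginPlay it binds Rewind and Forward to the player character and one TimeReverseEnemy, and these events toggle IsRewind.
; Disconnected logic would record the world transform into an array, then pop entries to reverse movement.
; Tick is empty, so recording and playback never run.
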(event `self.ReceiveBeginPlay`
  (`|ExecutionSequence`
    (:`then_0`
      (bind _returnvalue (`GameplayStatics.GetActorOfClass` "/Game/meshes/Superhot_Enemy_Stl/TimeReverseEnemy.TimeReverseEnemy_C"))
      (add `/Game/meshes/Superhot_Enemy_Stl/TimeReverseEnemy.Rewind` _returnvalue (delegate `Rewind`))
      (add `/Game/meshes/Superhot_Enemy_Stl/TimeReverseEnemy.Forward` _returnvalue (delegate `Forward`)))
    (:`then_1`
      (bind _asbp_first_person_character (cast `/Game/Blueprints/BP_FirstPersonCharacter` (`GameplayStatics.GetPlayerPawn` 0)))
      (add `/Game/Blueprints/BP_FirstPersonCharacter.Forward` _asbp_first_person_character (delegate `Forward`))
      (add `/Game/Blueprints/BP_FirstPersonCharacter.Rewind` _asbp_first_person_character (delegate `Rewind`)))))

(event `Rewind`
  (set `self.isRewind?` true))

(event `Forward`
  (set `self.isRewind?` false))

(event `self.ReceiveTick`
  (params (DeltaSeconds :type "Float (single-precision)"))
  ;[1 1 1] Time move
)