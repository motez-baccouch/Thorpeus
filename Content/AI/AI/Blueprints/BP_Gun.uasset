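; BP_Gun is a ranged weapon Blueprint with limited ammo, extending a parent that handles drop and pickup notification.
; Attack spawns a BP_Bullet at the Arrow component with an attached Niagara trail and a gunshot effect, then decrements Ammo.
; With no ammo left, Attack calls Drop instead, and pickup notifications reach the parent only while ammo remains.
; The Drop override calls the parent, followed by an empty zero-ammo check.
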(fn `Attack`
  (bind (_returnvalue_location _returnvalue_rotation) (`KismetMathLibrary.BreakTransform` (`SceneComponent.K2_GetComponentToWorld` (`self.Arrow`))))
  (if (> (`self.Ammo`) 0)
    (bind _returnvalue (`|SpawnActorFromClass` "/Game/AI/AI/Blueprints/BP_Bullet.BP_Bullet_C" (`KismetMathLibrary.MakeTransform` _returnvalue_location _returnvalue_rotation) "AlwaysSpawn" "OverrideRootScale" null null))
    (bind _output_get (set `self.NewVar_0` _returnvalue))
    (`NiagaraFunctionLibrary.SpawnSystemAttached` "/Game/VFX/BulletTrail_NS.BulletTrail_NS" (`/Game/AI/AI/Blueprints/BP_Bullet.StaticMesh` _output_get) "None" (0.0 0.0 0.0) (struct) "KeepRelativeOffset")
    (`NiagaraFunctionLibrary.SpawnSystemAtLocation` "/Game/AI/AI/N_GunShot.N_GunShot" (`SceneComponent.K2_GetComponentLocation` (`self.Arrow`)) (struct :`Roll` 90.0) (0.5 0.5 0.5))
    (set `self.Ammo` (- (`self.Ammo`) 1))
    (else
      (`self.Drop`))))

(fn `Drop`
  (`parent.Drop`)
  (if (== (`self.Ammo`) 0)
    _))

(fn `SendPickupNotification`
  (params (Enemy :type "/Game/AI/AI/Blueprints/BP_Enemy Object Reference"))
  (if (> (`self.Ammo`) 0)
    (`parent.SendPickupNotification` Enemy)))

(fn `UserConstructionScript`
  (`parent.UserConstructionScript`))