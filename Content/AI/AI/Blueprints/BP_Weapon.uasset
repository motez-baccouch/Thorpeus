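; BP_Weapon is a weapon actor that AI enemies can sight as a pickup, with an empty Attack function, likely for overriding.
; When a BP_Enemy enters VisionRange, it disables that range's overlap events and, if unattached, sets WeaponSighted and TargetWeapon on the enemy's Blackboard.
; Drop detaches it, enables mesh physics and applies a random impulse, without re-enabling overlap events.
; The out-of-sight notification logic exists but is disconnected.
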(event `self.VisionRange.OnComponentBeginOverlap`
  (params (OverlappedComponent :type "PrimitiveComponent Object Reference") (OtherActor :type "Actor Object Reference") (OtherComp :type "PrimitiveComponent Object Reference") (OtherBodyIndex :type Integer) (bFromSweep :type Boolean) (SweepResult :type "HitResult Structure (by ref)"))
  (if (== (`GameplayStatics.GetObjectClass` OtherActor) "/Game/AI/AI/Blueprints/BP_Enemy.BP_Enemy_C")
    (set `PrimitiveComponent.bGenerateOverlapEvents` false (`self.VisionRange`))
    (bind _asbp_enemy (cast `/Game/AI/AI/Blueprints/BP_Enemy` OtherActor))
    (`self.SendPickupNotification` _asbp_enemy)))

(event `self.VisionRange.OnComponentEndOverlap`
  (params (OverlappedComponent :type "PrimitiveComponent Object Reference") (OtherActor :type "Actor Object Reference") (OtherComp :type "PrimitiveComponent Object Reference") (OtherBodyIndex :type Integer)))

(fn `Attack`)

(fn `Drop`
  (bind _staticmesh (`self.StaticMesh`))
  (`SceneComponent.K2_DetachFromComponent` (`self.DefaultSceneRoot`) "KeepWorld" "KeepWorld" "KeepWorld" true)
  (`PrimitiveComponent.SetSimulatePhysics` _staticmesh true)
  (`PrimitiveComponent.AddImpulse` _staticmesh (`KismetMathLibrary.MakeVector` (* (`KismetMathLibrary.RandomFloat`) 10000.0) 0.0 (* (`KismetMathLibrary.RandomFloat`) 10000.0)) "None" false))

(fn `SendOutOfSightNotification`
  (params (Enemy :type "/Game/AI/AI/Blueprints/BP_Enemy Object Reference"))
  (`BlackboardComponent.SetValueAsBool` (`AIController.Blackboard` (`AIBlueprintHelperLibrary.GetAIController` Enemy)) "WeaponSighted" false))

(fn `SendPickupNotification`
  (params (Enemy :type "/Game/AI/AI/Blueprints/BP_Enemy Object Reference"))
  (bind _blackboard (`AIController.Blackboard` (`AIBlueprintHelperLibrary.GetAIController` Enemy)))
  (`/Engine/EditorBlueprintResources/StandardMacros.IsValid` (`SceneComponent.GetAttachParent` (`self.DefaultSceneRoot`))
    (:`Is Not Valid`
      (`BlackboardComponent.SetValueAsBool` _blackboard "WeaponSighted" true)
      (`BlackboardComponent.SetValueAsObject` _blackboard "TargetWeapon" self))))

(fn `UserConstructionScript`)