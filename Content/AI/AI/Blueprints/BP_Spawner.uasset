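; Timed enemy spawner that spawns BP_Enemy at random navmesh points around itself for a limited duration.
; BeginPlay derives EnemyCount from duration over interval, starts a looping spawn timer and a second timer that clears it.
; Each spawn plays a Niagara flash, but flash and enemy roll separate random points, so locations can differ.
; SpawnLevelEnd, not called here, spawns ChangeLevel_Bp near the player and passes it LevelName.
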(event `self.ReceiveBeginPlay`
  (set `self.EnemyCount` (`KismetMathLibrary.FTrunc` (/ (`self.TimeBeforeStoppingSpawn`) (`self.TimeBetweenSpawns`))))
  (bind _returnvalue (`KismetSystemLibrary.K2_SetTimerDelegate` (delegate `SpawnEnemy`) (`self.TimeBetweenSpawns`) true))
  (set `self.SpawnTimer` _returnvalue)
  (`KismetSystemLibrary.K2_SetTimerDelegate` (delegate `StopSpawning`) (`self.TimeBeforeStoppingSpawn`)))

(event `StopSpawning`
  (`KismetSystemLibrary.K2_ClearAndInvalidateTimerHandle` (`self.SpawnTimer`)))

(event `SpawnEnemy`
  (bind (_returnvalue_location _returnvalue_rotation) (`KismetMathLibrary.BreakTransform` (`self.GetTransform` self)))
  (bind _randomlocation (`NavigationSystemV1.K2_GetRandomLocationInNavigableRadius` _returnvalue_location 200.0 null null))
  (bind _returnvalue (`KismetMathLibrary.MakeVector` (.x _randomlocation) (.y _randomlocation) (+ (.z _randomlocation) 100.0)))
  (`NiagaraFunctionLibrary.SpawnSystemAtLocation` "/Game/AI/AI/Blueprints/NS_SpawnFlash.NS_SpawnFlash" _returnvalue _returnvalue_rotation)
  (`|SpawnActorFromClass` "/Game/AI/AI/Blueprints/BP_Enemy.BP_Enemy_C" (`KismetMathLibrary.MakeTransform` _returnvalue _returnvalue_rotation) "Undefined" "OverrideRootScale" null null))

(event `SpawnLevelEnd`
  (bind _returnvalue (`|SpawnActorFromClass` "/Game/Blueprints/VrBp/Blueprints/changeLevel_Bp.changeLevel_Bp_C" (`KismetMathLibrary.MakeTransform` (+ (`self.K2_GetActorLocation` (`GameplayStatics.GetPlayerPawn` 0)) (-100.0 0.0 100.0))) "Undefined" "OverrideRootScale" null null))
  (set `/Game/Blueprints/VrBp/Blueprints/changeLevel_Bp.levelName` (`self.Level Name`) _returnvalue))

(fn `UserConstructionScript`)