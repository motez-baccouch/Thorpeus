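; AI enemy character that fights unarmed or with an equipped weapon.
; Equip, pickup, drop and stun logic write the combat state enum to the AI controller's Blackboard, separating guns from other weapons.
; Attack delegates to the held weapon or plays a random unarmed montage.
; A first-person projectile hit destroys the capsule and mesh and spawns a short-lived Enemy1 actor from the capsule's relative transform.
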(event `self.ReceiveBeginPlay`
  (bind _blackboard (`AIController.Blackboard` (`AIBlueprintHelperLibrary.GetAIController` self)))
  (bind _blackboard_2 (`AIController.Blackboard` (`AIBlueprintHelperLibrary.GetAIController` self)))
  (if (`self.IsEquipped`)
    ;[1 1 1] Attach Weapon & Set Equipped Params
    (bind _returnvalue (`|SpawnActorFromClass` (`self.Weapon`) (`self.Weapon Spawn Transform`) "AlwaysSpawn" "OverrideRootScale" null null))
    (bind _output_get (set `self.EquippedWeapon` _returnvalue))
    (`self.K2_AttachToComponent` _output_get (`self.Mesh`) "RightHandWeaponSocket" "SnapToTarget" "SnapToTarget" "SnapToTarget" true)
    (`BlackboardComponent.SetValueAsBool` _blackboard "IsEquipped" (`self.IsEquipped`))
    (if (== (`GameplayStatics.GetObjectClass` (`self.EquippedWeapon`)) "/Game/AI/AI/Blueprints/BP_Gun.BP_Gun_C")
      (bind _output_get_2 (set `self.CurrentState` "NewEnumerator2"))
      (`BlackboardComponent.SetValueAsEnum` _blackboard "CurrentState" _output_get_2)
      (else
        (bind _output_get_3 (set `self.CurrentState` "NewEnumerator1"))
        (`BlackboardComponent.SetValueAsEnum` _blackboard "CurrentState" _output_get_3)))
    (else
      ;[1 1 1] Set Unequipped Params
      (`BlackboardComponent.SetValueAsBool` _blackboard_2 "IsEquipped" (`self.IsEquipped`))
      (bind _output_get_4 (set `self.CurrentState` "NewEnumerator0"))
      (`BlackboardComponent.SetValueAsEnum` _blackboard_2 "CurrentState" _output_get_4))))

(event `Attack`
  (if (`self.IsEquipped`)
    ;[1 1 1] Ranged Attack
    (`/Game/AI/AI/Blueprints/BP_Weapon.Attack` (`self.EquippedWeapon`))
    (else
      ;[1 1 1] Melee Attack
      (`|PlayMontage` (`self.Mesh`) (select `int` (`KismetMathLibrary.RandomIntegerInRange` 0 3) :`0` "/Game/AI/AI/Animation/Animations/StandardAttack_Montage.StandardAttack_Montage" :`1` "/Game/AI/AI/Animation/Animations/Punch_Montage.Punch_Montage" :`2` "/Game/AI/AI/Animation/Animations/UpAttack_Montage.UpAttack_Montage" :!type "AnimMontage Object Reference")))))

(event `GetStunned`
  (bind _output_get (set `self.CurrentState` "NewEnumerator3"))
  (`BlackboardComponent.SetValueAsEnum` (`AIController.Blackboard` (`AIBlueprintHelperLibrary.GetAIController` self)) "CurrentState" _output_get))

(event `self.ReceiveHit`
  (params (MyComp :type "PrimitiveComponent Object Reference") (Other :type "Actor Object Reference") (OtherComp :type "PrimitiveComponent Object Reference") (bSelfMoved :type Boolean) (HitLocation :type "Vector Structure") (HitNormal :type "Vector Structure") (NormalImpulse :type "Vector Structure") (Hit :type "HitResult Structure (by ref)"))
  (bind _capsulecomponent (`self.CapsuleComponent`))
  (if (== (`GameplayStatics.GetObjectClass` Other) "/Game/Blueprints/BP_FirstPersonProjectile.BP_FirstPersonProjectile_C")
    (bind _output_get (set `self.MannequinTransform` (`SceneComponent.GetRelativeTransform` _capsulecomponent)))
    (`ActorComponent.K2_DestroyComponent` _capsulecomponent)
    (`ActorComponent.K2_DestroyComponent` (`self.Mesh`))
    (bind _returnvalue (`|SpawnActorFromClass` "/Game/meshes/Superhot_Enemy_Stl/enemy1.enemy1_C" _output_get "Undefined" "OverrideRootScale" null null))
    (bind _output_get_2 (set `self.NewVar_1` _returnvalue))
    (`KismetSystemLibrary.Delay` 2.0)
    (`self.K2_DestroyActor` _output_get_2)))

(fn `DropWeapon`
  (bind _blackboard (`AIController.Blackboard` (`AIBlueprintHelperLibrary.GetAIController` self)))
  (bind _output_get (set `self.IsEquipped` false))
  (`BlackboardComponent.SetValueAsBool` _blackboard "WeaponSighted" true)
  (`BlackboardComponent.SetValueAsBool` _blackboard "IsEquipped" _output_get)
  (`/Game/AI/AI/Blueprints/BP_Weapon.Drop` (`self.EquippedWeapon`))
  (`self.UpdateBBCurrentState` "NewEnumerator0"))

(fn `PickupWeapon`
  (bind _returnvalue (`GameplayStatics.GetObjectClass` (`self.EquippedWeapon`)))
  (bind _outactors (`GameplayStatics.GetAllActorsOfClass` "/Game/AI/AI/Blueprints/BP_Weapon.BP_Weapon_C"))
  (for _array_element _outactors
    (bind _output_get (set `self.EquippedWeapon` _array_element))
    (if (`PrimitiveComponent.IsOverlappingComponent` (`self.CapsuleComponent`) (`/Game/AI/AI/Blueprints/BP_Weapon.PickupRange` _output_get))
      (`self.K2_AttachToComponent` _array_element (`self.Mesh`) "RightHandWeaponSocket" "SnapToTarget" "SnapToTarget" "SnapToTarget" true)
      (set `self.IsEquipped` true)
      (if (== _returnvalue "/Game/AI/AI/Blueprints/BP_Gun.BP_Gun_C")
        (set `self.CurrentState` "NewEnumerator2")
        (`BlackboardComponent.SetValueAsEnum` (`AIController.Blackboard` (`AIBlueprintHelperLibrary.GetAIController` self)) "CurrentState" (stale _output_get_2) :!label _label)
        (elif (== _returnvalue "/Game/AI/AI/Blueprints/BP_Melee.BP_Melee_C")
          (bind _output_get_2 (set `self.CurrentState` "NewEnumerator1"))
          (goto _label))))))

(fn `UpdateBBCurrentState`
  (params (CurrentState :type "/Game/AI/AI/ENUM_EnemyState Enum" :default "NewEnumerator0"))
  (bind _output_get (set `self.CurrentState` CurrentState))
  (`BlackboardComponent.SetValueAsEnum` (`AIController.Blackboard` (`AIBlueprintHelperLibrary.GetAIController` self)) "CurrentState" _output_get))

(fn `UserConstructionScript`)