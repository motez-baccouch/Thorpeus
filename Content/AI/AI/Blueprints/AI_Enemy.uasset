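; AI controller for enemies that starts the BT_Enemy behavior tree when it possesses a pawn.
; After a short delay, it stores the first player's pawn as the TargetPlayer blackboard object and enables ticking on the possessed pawn.
; Every tick, it derives the IsWeaponPickable blackboard flag, true when a weapon is sighted and none is equipped.
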(event `self.ReceivePossess`
  (params (PossessedPawn :type "Pawn Object Reference"))
  (`self.RunBehaviorTree` "/Game/AI/AI/BT_Enemy.BT_Enemy")
  (`KismetSystemLibrary.Delay` 0.2)
  (`BlackboardComponent.SetValueAsObject` (`self.Blackboard`) "TargetPlayer" (`GameplayStatics.GetPlayerPawn` 0))
  (`self.SetActorTickEnabled` PossessedPawn true))

(event `self.ReceiveTick`
  (params (DeltaSeconds :type "Float (single-precision)"))
  (`BlackboardComponent.SetValueAsBool` (`self.Blackboard`) "IsWeaponPickable" (and (not (`self.GetBBBoolKey` (`self.IsEquippedKeyName`))) (`self.GetBBBoolKey` (`self.IsWeaponSightedKeyName`)))))

(fn `UserConstructionScript`)