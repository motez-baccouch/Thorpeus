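; Shuriken projectile Blueprint in the VR Blueprints folder that triggers a field and a burst effect on impact, then destroys itself.
; On hit, the AddForce1 event spawns an FS_MasterField actor at the shuriken's transform, and a RadialBurst system spawns at the hit location.
; A physics impulse branch is left unconnected, and the AddForce function is an empty stub.
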(event `self.ReceiveHit`
  (params (MyComp :type "PrimitiveComponent Object Reference") (Other :type "Actor Object Reference") (OtherComp :type "PrimitiveComponent Object Reference") (bSelfMoved :type Boolean) (HitLocation :type "Vector Structure") (HitNormal :type "Vector Structure") (NormalImpulse :type "Vector Structure") (Hit :type "HitResult Structure (by ref)"))
  (`self.AddForce1` (`self.GetTransform`))
  (`NiagaraFunctionLibrary.SpawnSystemAtLocation` "/Niagara/DefaultAssets/Templates/Systems/RadialBurst.RadialBurst" HitLocation)
  (`self.K2_DestroyActor`) ; Then destroy this projectile
)

(event `AddForce1`
  (params (NewParam :type "Transform Structure"))
  (`|SpawnActorFromClass` "/Engine/EditorResources/FieldNodes/FS_MasterField.FS_MasterField_C" NewParam "Undefined" "OverrideRootScale" null null))

(fn `addForce`
  (params (SpawnTransform1 :type "Transform Structure")))

(fn `UserConstructionScript`)